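; BP_Interactable is a prototype interactable actor that shows a widget and responds to the E key while the player character is nearby.
; WidgetTrigger overlaps with BP_Character set IsInside, toggle the widget's visibility and enable the actor's input on entry.
; On exit, DisableInput targets the player controller rather than the actor.
; Pressing E while inside only prints a debug message.
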(event OnComponentBeginOverlap(WidgetTrigger)
  (params (OverlappedComponent :type Primitive%20Component%20Object%20Reference) (OtherActor :type Actor%20Object%20Reference) (OtherComp :type Primitive%20Component%20Object%20Reference) (OtherBodyIndex :type Integer) (bFromSweep :type Boolean) (SweepResult :type Hit%20Result%20Structure%20%28by%20ref%29))
  (bind _asbp_character (Utilities|Casting|CastToBP_Character OtherActor))
  (Variables|Default|SetisInside true)
  (Input|EnableInput (Game|GetPlayerController 0))
  (Rendering|SetVisibility (Variables|Default|GetWidget) true false))

(event OnComponentEndOverlap(WidgetTrigger)
  (params (OverlappedComponent :type Primitive%20Component%20Object%20Reference) (OtherActor :type Actor%20Object%20Reference) (OtherComp :type Primitive%20Component%20Object%20Reference) (OtherBodyIndex :type Integer))
  (Utilities|Casting|CastToBP_Character OtherActor)
  (Variables|Default|SetisInside false)
  (Input|DisableInput (Game|GetPlayerController 0) 0)
  (Rendering|SetVisibility (Variables|Default|GetWidget) false false))

(event EventTick
  (params (DeltaSeconds :type Float%20%28single-precision%29)))

(event Input|KeyboardEvents|E
  (params (Key :type Key%20Structure :default "None"))
  (:Pressed
    (if (Variables|Default|GetisInside)
      (Development|PrintString "Kliknieto E"))))

(fn ConstructionScript)

(fn NewFunction)