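; BP_ItemSpawner is an actor that scatters potion pickups throughout a box area when play begins.
; On BeginPlay, a fixed-count loop spawns a mana potion, a health potion and a bad health potion on each pass.
; Each spawn gets its own random point inside the SpawnArea box, computed from that component's world location and scaled extent.
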(event Collision|EventActorBeginOverlap
  (params (OtherActor :type Actor%20Object%20Reference)))

(event EventTick
  (params (DeltaSeconds :type Float%20%28single-precision%29)))

(event EventBeginPlay
  (bind _spawnarea (Variables|Default|GetSpawnArea))
  (bind _spawnarea_2 (Variables|Default|GetSpawnArea))
  (bind _spawnarea_3 (Variables|Default|GetSpawnArea))
  (for _index (range 0 15)
    (Game|SpawnActorfromClass "/Game/Lab1/ManaPotion.ManaPotion_C" (Math|Transform|MakeTransform (Math|Random|RandomPointinBoundingBox (Transformation|GetWorldLocation _spawnarea_2) (Components|Box|GetScaledBoxExtent _spawnarea_2)) "0, 0, 0" "1.000000,1.000000,1.000000") "Undefined" "MultiplyWithRoot" 0 0)
    (Game|SpawnActorfromClass "/Game/Lab1/HealthPotion.HealthPotion_C" (Math|Transform|MakeTransform (Math|Random|RandomPointinBoundingBox (Transformation|GetWorldLocation _spawnarea_3) (Components|Box|GetScaledBoxExtent _spawnarea_3)) "0, 0, 0" "1.000000,1.000000,1.000000") "Undefined" "MultiplyWithRoot" 0 0)
    (Game|SpawnActorfromClass "/Game/Lab1/Potions/BadHealthPotion.BadHealthPotion_C" (Math|Transform|MakeTransform (Math|Random|RandomPointinBoundingBox (Transformation|GetWorldLocation _spawnarea) (Components|Box|GetScaledBoxExtent _spawnarea)) "0, 0, 0" "1.000000,1.000000,1.000000") "Undefined" "MultiplyWithRoot" 0 0)))

(fn ConstructionScript)