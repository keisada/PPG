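; BP_NPC is an NPC Blueprint that shows its name and health through widget components.
; On BeginPlay it casts the Name component's widget to W_NPC_Name and sets its text from NPCName.
; It then casts the Health component's widget to NPC_HealthBar and sets the bar percent from NPCHealth.
; Both values are written only at BeginPlay in this graph, and a failed cast stops the sequence.
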(event EventBeginPlay
  (bind _asw_npc_name (Utilities|Casting|CastToW_NPC_Name (UserInterface|GetUserWidgetObject (Variables|Default|GetName))))
  (Variables|/Script/UMG.TextBlock|SetText (Variables|/Game/NPC/W_NPC_Name.W_NPC_Name_C|GetNPC_Name _asw_npc_name) (Utilities|Text|ToText(String) (Variables|Default|GetNPC_Name)))
  (bind _asnpc_health_bar (Utilities|Casting|CastToNPC_HealthBar (UserInterface|GetUserWidgetObject (Variables|Default|Gethealth))))
  (Progress|SetPercent (Variables|/Game/NPC/NPC_HealthBar.NPC_HealthBar_C|GetNPC_Health _asnpc_health_bar) (Variables|Default|GetNPC_Health)))

(fn ConstructionScript)